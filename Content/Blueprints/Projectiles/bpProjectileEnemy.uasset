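; bpProjectileEnemy is an enemy projectile that damages the player on contact.
; Tick moves it by a local offset of Speed scaled by delta time, without sweeping.
; When its mesh begins overlapping any actor it destroys itself, applying Damage first only if that actor is a bpPlayer.
; The construction script sets the actor's size from its Scale variable.
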(event OnComponentBeginOverlap(ProjectileMesh)
  (params (OverlappedComponent :type Primitive%20Component%20Object%20Reference) (OtherActor :type Actor%20Object%20Reference) (OtherComp :type Primitive%20Component%20Object%20Reference) (OtherBodyIndex :type Integer) (bFromSweep :type Boolean) (SweepResult :type Hit%20Result%20Structure%20%28by%20ref%29))
  ;[1 1 1] Collision Events
  (bind _asbp_player (Utilities|Casting|CastTobpPlayer OtherActor)
    (:then
      (Game|Damage|ApplyDamage _asbp_player (Variables|Default|Getdamage) 0 0))
    (:CastFailed
      _))
  (Actor|DestroyActor))

(event EventTick
  (params (DeltaSeconds :type Float%20%28single-precision%29))
  ;[1 1 1] Move Projectile
  (Transformation|AddActorLocalOffset (* (Variables|Default|Getspeed) DeltaSeconds) false false))

(fn ConstructionScript
  (Transformation|SetActorScale3D (Variables|Default|Getscale)))