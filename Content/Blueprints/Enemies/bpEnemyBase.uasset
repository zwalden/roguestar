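; Base enemy actor that slides in on spawn, moves along Z and damages the player on contact.
; BeginPlay registers it in bpGameMode's LiveEnemies and randomizes direction, speed and entry distance; a timeline lerps it along -Y before enabling swept Tick movement.
; Non-enemy hits set direction from negated IsMoveEnabled, rather than toggling it.
; AnyDamage sets Health to clamped Damage minus Health, and at zero decrements LiveEnemies and destroys the actor.
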(event EventBeginPlay
  ;[1 1 1] Control Random Enemy Projectile Config
  (bind _asbp_game_mode (Utilities|Casting|CastTobpGameMode (Game|GetGameMode)))
  (bind _output_get (Variables|Default|SetbpGameMode _asbp_game_mode))
  (Variables|/Game/Blueprints/bpGameMode.bpGameMode_C|SetliveEnemies _output_get (+ (Variables|/Game/Blueprints/bpGameMode.bpGameMode_C|GetliveEnemies _output_get) 1))
  (Variables|Default|SetbMoveDirection (Math|Random|RandomBool))
  (Variables|Float|SetmoveSpeed (Math|Random|RandomFloatinRange 5e+02 1e+03))
  (Variables|Float|SetsweepIn (Math|Random|RandomFloatinRange 1.2e+03 1.7e+03))
  ;[1 1 1] Spawn Animation
  (Variables|Default|SetspawnLocation (Transformation|GetActorLocation))
  (bind _speed (Timeline|SpawnAnimation Play)
    (:Update
      (Transformation|SetActorLocation (Math|Vector|Lerp(Vector) (Variables|Default|GetspawnLocation) (- (Variables|Default|GetspawnLocation) (Math|Vector|MakeVector 0.0 (Variables|Float|GetsweepIn) 0.0)) _speed) false false))
    (:Finished
      (Variables|Default|SetbIsMoveEnabled true))))

(event EventTick
  (params (DeltaSeconds :type Float%20%28single-precision%29))
  ;[1 1 1] Movement
  (if (Variables|Default|GetbIsMoveEnabled)
    (Transformation|SetActorLocation (+ (Transformation|GetActorLocation) (* (Math|Vector|RotateVector (Math|Vector|MakeVector 0.0 0.0 (* (Variables|Float|GetmoveSpeed) (Math|Float|SelectFloat 1.0 -1.0 (Variables|Default|GetbMoveDirection)))) "0, 0, 0") DeltaSeconds)) true false)))

(event Collision|EventHit
  (params (MyComp :type Primitive%20Component%20Object%20Reference) (Other :type Actor%20Object%20Reference) (OtherComp :type Primitive%20Component%20Object%20Reference) (bSelfMoved :type Boolean) (HitLocation :type Vector :default "0, 0, 0") (HitNormal :type Vector :default "0, 0, 0") (NormalImpulse :type Vector :default "0, 0, 0") (Hit :type Hit%20Result%20Structure%20%28by%20ref%29))
  ;[1 1 1] Enemy Death
  (Utilities|Casting|CastTobpEnemyBase Other
    (:CastFailed
      (Variables|Default|SetbMoveDirection (not (Variables|Default|GetbIsMoveEnabled)))
      (bind _asbp_player (Utilities|Casting|CastTobpPlayer Other))
      (Game|Damage|ApplyDamage _asbp_player 5e+01 0 0))))

(event Game|Damage|EventAnyDamage
  (params (Damage :type Float%20%28single-precision%29) (DamageType :type Damage%20Type%20Object%20Reference) (InstigatedBy :type Controller%20Object%20Reference) (DamageCauser :type Actor%20Object%20Reference))
  (bind _bpgamemode (Variables|Default|GetbpGameMode))
  ;[1 1 1] Enemy Death
  (Variables|Float|Sethealth (Math|Float|Clamp(Float) (- Damage (Variables|Float|Gethealth)) 0.0 (Variables|Float|GetmaxHealth)))
  (if (<= (Variables|Float|Gethealth) 0.0)
    (Variables|/Game/Blueprints/bpGameMode.bpGameMode_C|SetliveEnemies _bpgamemode (- (Variables|/Game/Blueprints/bpGameMode.bpGameMode_C|GetliveEnemies _bpgamemode) 1))
    (Actor|DestroyActor)))

(fn ConstructionScript
  (Variables|Float|Sethealth (Variables|Float|GetmaxHealth)))